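; Melee weapon block ability that applies a blocking gameplay effect to its owner.
; After a cost check and short fixed delay, it applies the effect, then watches for input release and attribute changes, intended to detect health loss.
; Release ends the ability without committing, while an attribute decrease commits cost and cooldown before ending.
; Ending the ability removes the effect through its stored handle.
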(event `self.K2_ActivateAbility`
  ;[1 1 1] Apply blocking GE until health goes down or block input is released
  (bind _returnvalue (`self.K2_CheckAbilityCost`))
  (if _returnvalue
    (`AbilityTask_WaitDelay.WaitDelay` 0.4 ; Could use anim notify for this
      (:`OnFinish`
        (bind _returnvalue_2 (`self.BP_ApplyGameplayEffectToOwner` (`self.BlockingEffect`)))
        (set `self.BlockingHandle` _returnvalue_2)
        (bind (_asynctaskproxy _attribute _newvalue _oldvalue) (`AbilityAsync_WaitAttributeChanged.WaitForAttributeChanged` (`self.GetOwningActorFromActorInfo`) (struct :`AttributeName` "Health" :`Attribute` "/Script/NarrativeArsenal.NarrativeAttributeSetBase:Health" :`AttributeOwner` "/Script/CoreUObject.Class'/Script/NarrativeArsenal.NarrativeAttributeSetBase'"))
          (:`then`
            (bind _asynctaskproxy_2 (`AbilityTask_WaitInputRelease.WaitInputRelease` true)
              (:`then`
                (set `self.WaitInputRelease` _asynctaskproxy_2))
              (:`OnRelease`
                (`self.K2_EndAbility`))))
          (:`Changed`
            (if (< _newvalue _oldvalue)
              (`self.K2_CommitAbility`)
              (`self.K2_EndAbility`))))))))

(event `self.K2_OnEndAbility`
  (params (bWasCancelled :type Boolean))
  ;[1 1 1] Remove blocking effect
  (`self.BP_RemoveGameplayEffectFromOwnerWithHandle` (`self.BlockingHandle`)))

(fn `K2_CanActivateAbility`
  (params (ActorInfo :type "GameplayAbilityActorInfo Structure") (Handle :type "GameplayAbilitySpecHandle Structure"))
  (returns (RelevantTags :type "GameplayTagContainer Structure") (ReturnValue :type Boolean))
  (return (struct) true))