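; Interact ability that lets a character mount a pawn such as a car or horse as driver or passenger, including carjacking the occupant.
; It moves to the slot, motion-warps montages into the seat alongside door animations, then attaches and possesses the mount (passengers only ignore move input).
; Exiting unpossesses and warps out to a floor-traced spot, while stolen occupants await a Carjacked event, then ragdoll.
; Ability end restores walking, collision and animation state.
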(event `self.HandleInteraction`
  (params (bIsStealing :type Boolean) (StealingFrom :type "NarrativeInteractionComponent Object Reference"))
  (bind (_returnvalue_location _returnvalue_rotation) (`KismetMathLibrary.BreakTransform` (`KismetMathLibrary.ComposeTransforms` (`.SlotTransform` (break `InteractionSlotConfig` (`self.SlotConfiguration`))) (`Actor.GetTransform` (`self.PawnToMount`)))))
  (bind (_returnvalue_location_2 _returnvalue_rotation_2) (`KismetMathLibrary.BreakTransform` (`KismetMathLibrary.ComposeTransforms` (`KismetMathLibrary.MakeTransform` (* (.location (`/Game/Abilities/GameplayAbilities/Interacts/Mount/BP_SlotBehavior_Mount.GetOutTransform` (`self.MountBehavior`))) (2.0 2.0 1.0)) (.rotation (`/Game/Abilities/GameplayAbilities/Interacts/Mount/BP_SlotBehavior_Mount.GetOutTransform` (`self.MountBehavior`))) (.scale (`/Game/Abilities/GameplayAbilities/Interacts/Mount/BP_SlotBehavior_Mount.GetOutTransform` (`self.MountBehavior`)))) (`Actor.GetTransform` (`self.PawnToMount`)))))
  ;[0 0.3246 1] STEP 1: To mount something, we walk to the right spot, play a motion warped animation, and notify once we're in place.
  ; This has been complicated a bit since mount stealing has been added - we also "throw" the occupant off the mount if we're stealing the mount. I believe ContextualAnimations could clean this up a bit in future
  ;; A. Set up state, and move to the get in transform
  (bind _succeeded (`self.Grab Mount Data` StealingFrom))
  (if _succeeded
    (set `self.MovingToLocation` true)
    (`GameplayTask_MoveToLocationAndRotation.MoveToLocationAndRotation` null _returnvalue_location _returnvalue_rotation 90.0
      (:`OnCompleted`
        ;; B. Start driver get in montage, and open the cars door
        (set `self.MovingToLocation` false)
        (bind _returnvalue (`NarrativeAbilitySystemComponent.AddDynamicTagsGameplayEffect` (`NarrativeCharacter.AbilitySystemComponent` (`self.CharacterOwner`)) (`BlueprintGameplayTagLibrary.MakeLiteralGameplayTagContainer` (struct :`GameplayTags` (struct :`(TagName` "Camera.FirstPerson.Follow3PHeadLocation") :`(TagName` "Camera.FirstPerson.Follow3PHeadRotation") :`(TagName` "Camera.FirstPerson.DisableFirstPersonRendering") :`(TagName` "Narrative.State.OnMount")))))) ; required to make FP anims feel nice when entering
        (set `self.DynamicTagsForEntry` _returnvalue)
        (`AbilityTask_PlayMontageAndWait.CreatePlayMontageAndWaitProxy` "None" (`self.Get Driver Get In Montage`)
          (:`then`
            (`self.Started Entry Warp`)
            (`|PlayMontage` (`self.GetMountSkeletalMesh` (`self.PawnToMount`)) (`self.Get Mount Driver Get In Montage`)
              (:`then`
                ;; Carjack the existing occupant if needed
                (bind _stealingfrompawn (`self.StealingFromPawn`) ; add this back in when we go contexual
                  (:`then`
                    (`NarrativeAnimInstance.RemoveOverrideLayer` (`NarrativeCharacter.GetCharacterAnimInstance` _stealingfrompawn) 0.0)
                    (`|PlayMontage` (`Character.Mesh` (`self.StealingFromPawn`)) (`self.Get Mount Driver Thrown Out Montage`) ; If we're carjacking, pull existing driver out
                      (:`then`
                        (`self.Ready Character For Warping` (`self.StealingFromPawn`))
                        (`MotionWarpingComponent.AddOrUpdateWarpTargetFromTransform` (`NarrativeCharacter.MotionWarpingComponent` (`self.StealingFromPawn`)) (`/Game/Abilities/GameplayAbilities/Interacts/Mount/BP_SlotBehavior_Mount.SitMontageWarpTargetName` (`self.MountBehavior`)) (`KismetMathLibrary.MakeTransform` (`self.FindFloor` _returnvalue_location_2) _returnvalue_rotation_2)) ; Go back to the stand up spot
                      )))
                  (:`else`
                    _))
                ;; Warp the driver into the drivers seat
                (`self.Ready Character For Warping` (`self.CharacterOwner`))
                (`MotionWarpingComponent.AddOrUpdateWarpTargetFromComponent` :`self` (`NarrativeCharacter.MotionWarpingComponent` (`self.CharacterOwner`)) :`WarpTargetName` (`/Game/Abilities/GameplayAbilities/Interacts/Mount/BP_SlotBehavior_Mount.SitMontageWarpTargetName` (`self.MountBehavior`)) :`Component` (`self.GetMountSkeletalMesh` (`self.PawnToMount`)) :`BoneName` (`/Game/Abilities/GameplayAbilities/Interacts/Mount/BP_SlotBehavior_Mount.SeatSocketName` (`self.MountBehavior`)) :`bFollowComponent` true :`LocationOffset` (`KismetMathLibrary.MakeVector` 0.0 0.0 (* (+ (`CapsuleComponent.GetScaledCapsuleHalfHeight` (`Character.CapsuleComponent` (`self.CharacterOwner`))) 2.0) -1.0))))))
          (:`OnBlendOut`
            (`self.Finished Entry Warp`)
            (`self.On Entered Seat`))))
      (:`OnFailed`
        (`GameplayTask_WaitDelay.TaskWaitDelay` null 0.1
          (:`OnFinish`
            (set `self.MovingToLocation` false)
            (`self.K2_EndAbility`)))))
    (else
      (`self.K2_EndAbility`))))

(event `On Entered Seat`
  ;[0.0172 0.15 0] STEP 2: We're in place - possess the mount, and attach our bipedal character to it.
  (`Actor.K2_AttachToComponent` (`self.OldCharacter`) (`self.GetMountSkeletalMesh` (`self.PawnToMount`)) (`/Game/Abilities/GameplayAbilities/Interacts/Mount/BP_SlotBehavior_Mount.SeatSocketName` (`self.MountBehavior`)) "SnapToTarget" "SnapToTarget" "KeepWorld" false)
  ;; Either possess the car or just make it our view target if we're a passenger
  (`self.PossessMount`))

(event `self.FinishInteraction`
  (params (bWasStolen :type Boolean))
  (bind (_returnvalue_location _returnvalue_rotation) (`KismetMathLibrary.BreakTransform` (`KismetMathLibrary.ComposeTransforms` (`/Game/Abilities/GameplayAbilities/Interacts/Mount/BP_SlotBehavior_Mount.GetOutTransform` (`self.MountBehavior`)) (`Actor.GetTransform` (`self.PawnToMount`)))))
  ;[1 0.3049 0] STEP 3: When we finish up, play the get up montage and then end ability
  (if (`NarrativeCharacter.IsAlive` (`self.OldCharacter`))
    (bind _output_get (set `self.WeWereStolen` bWasStolen))
    (if _output_get
      (`KismetSystemLibrary.PrintString` "we got stolen!" false false) ; If we were stolen, stealer is going to animate us being thrown out of the car - we need to keep all our settings until that is done.\nWe could use an event notify to wait until they throw us out, but this is already getting quite complex and could get out of hand - keep it simple with a delay that restores our state without actually playing the get out animation.
      (`AbilityTask_WaitGameplayEvent.WaitGameplayEvent` (struct :`TagName` "GameplayEvent.WantsEndInteract.Carjacked") null
        (:`EventReceived`
          (`NarrativeCharacter.RagdollForDuration` (`self.CharacterOwner`) 4.0)
          (`self.UnpossessMount`)
          (`KismetSystemLibrary.PrintString` "restoring state after we got jacked" false false)
          (`self.K2_EndAbility`) ; Since jacker handled throwing us out of the car, we can just end ability to restore all our settings
        ))
      (else
        (`KismetSystemLibrary.PrintString` "ending, but not stolen" false false)
        (`self.UnpossessMount`)
        (`self.Ready Character For Warping` (`self.OldCharacter`))
        (if (`self.MovingToLocation`)
          (`self.K2_EndAbility`)
          (elif (not (`self.StartedFinish?`))
            (set `self.StartedFinish?` true)
            (`AbilityTask_PlayMontageAndWait.CreatePlayMontageAndWaitProxy` "None" (`self.Get Driver Get Out Montage`)
              (:`then`
                (if (not (`self.WeWereStolen`))
                  (`|PlayMontage` (`self.GetMountSkeletalMesh` (`self.PawnToMount`)) (`/Game/Abilities/GameplayAbilities/Interacts/Mount/BP_SlotBehavior_Mount.Car_OpenDoor_GetOut` (`self.MountBehavior`))
                    (:`then`
                      _)))
                (`self.Started Exit Warp`)
                (bind _returnvalue (message `NarrativeCharacterOwner.GetNarrativeCharacter` (`self.OldController`)))
                (`NarrativeAnimInstance.RemoveOverrideLayer` (`NarrativeCharacter.GetCharacterAnimInstance` _returnvalue) 0.0)
                (`MotionWarpingComponent.AddOrUpdateWarpTargetFromTransform` (`NarrativeCharacter.MotionWarpingComponent` (`self.OldCharacter`)) (`/Game/Abilities/GameplayAbilities/Interacts/Mount/BP_SlotBehavior_Mount.SitMontageWarpTargetName` (`self.MountBehavior`)) (`KismetMathLibrary.MakeTransform` (`self.FindFloor` _returnvalue_location) _returnvalue_rotation)) ; Go back to the stand up spot
              )
              (:`OnCompleted`
                (`self.Finished Exit Warp`)
                (`self.K2_EndAbility`))
              (:`OnInterrupted`
                (`self.K2_EndAbility` :!label _label))
              (:`OnCancelled`
                (goto _label)))))))
    (else
      (`self.K2_EndAbility`) ; If we died immediately end
      (`KismetSystemLibrary.PrintString` "killed, ending ability" false false))))

(event `self.K2_OnEndAbility`
  (params (bWasCancelled :type Boolean))
  (bind _returnvalue (`NarrativeCharacter.GetCharacterAnimInstance` (`self.CharacterOwner`)))
  ;[1 0.1405 0] STEP 4: Final cleanup
  (`self.Restore Character From Warping` (`self.CharacterOwner`)) ; Ensure when ability ends we're always back into walking
  (if (== (`NarrativeAnimInstance.CurrentOverrideLayer` _returnvalue) (struct :`TagName` "Narrative.Anim.OverrideLayer.Driving"))
    (`NarrativeAnimInstance.RemoveOverrideLayer` _returnvalue 0.0))
  (`AbilitySystemComponent.RemoveActiveGameplayEffect` (`NarrativeCharacter.AbilitySystemComponent` (`self.CharacterOwner`)) (`self.DynamicTagsForEntry`) -1)
  (bind _movetolocationtask (`self.MoveToLocationTask`)
    (:`then`
      (`GameplayTask.EndTask` _movetolocationtask))
    (:`else`)))

(fn `CanExitInteraction`
  (params (bBeingStolen :type Boolean))
  (returns (ReturnValue :type Boolean))
  (bind _returnvalue (message `NarrativeCharacterOwner.GetNarrativeCharacter` (`self.OldController`)))
  (if (`NarrativeCharacter.IsAlive` _returnvalue)
    (return (and (or (== (`Controller.K2_GetPawn` (`self.OldController`)) (`self.PawnToMount`)) (== (`Actor.GetAttachParentActor` _returnvalue) (`self.PawnToMount`))) (< (`KismetMathLibrary.VSize` (`Actor.GetVelocity` (`self.PawnToMount`))) 50.0))) ; If we're entering/exiting sitting, dont allow us to get up yet.\nAlso dont let us exit moving mounts, as having anims etc for this would be quite diifficult
    (else
      (return true) ; Can always exit if we've been killed - build this into base
    )))

(fn `FindFloor`
  (params (Loc :type "Vector Structure"))
  (returns (ImpactPoint :type "Vector Structure"))
  (bind (_outhit _returnvalue) (`KismetSystemLibrary.LineTraceSingleForObjects` (+ Loc (0.0 0.0 20.0)) (- Loc (0.0 0.0 20.0)) (`|MakeArray` "ObjectTypeQuery1" "ObjectTypeQuery2" :!type "EObjectTypeQuery Enum") true))
  (if _returnvalue
    (return (`.ImpactPoint` (`GameplayStatics.BreakHitResult` _outhit)))
    (else
      (return (`local.Loc`)))))

(fn `Finished Entry Warp`)

(fn `Finished Exit Warp`)

(fn `Get Driver Get In Montage`
  (returns (Character_GetOnMount :type "AnimMontage Object Reference"))
  (bind _mountbehavior (`self.MountBehavior`))
  (`self.StealingFromPawn`
    (:`then`
      (return (`/Game/Abilities/GameplayAbilities/Interacts/Mount/BP_SlotBehavior_Mount.Character_Carjack_Steal` _mountbehavior)))
    (:`else`
      (return (`/Game/Abilities/GameplayAbilities/Interacts/Mount/BP_SlotBehavior_Mount.Character_GetOnMount` _mountbehavior)))))

(fn `Get Driver Get Out Montage`
  (returns (Character_GetOnMount :type "AnimMontage Object Reference"))
  (return (`/Game/Abilities/GameplayAbilities/Interacts/Mount/BP_SlotBehavior_Mount.Character_GetOffMount` (`self.MountBehavior`))))

(fn `Get Mount Driver Get In Montage`
  (returns (Car_GetInMontage :type "AnimMontage Object Reference"))
  (bind _mountbehavior (`self.MountBehavior`))
  (`self.StealingFromPawn`
    (:`then`
      (return (`/Game/Abilities/GameplayAbilities/Interacts/Mount/BP_SlotBehavior_Mount.Car_OpenDoor_Carjack` _mountbehavior)))
    (:`else`
      (return (`/Game/Abilities/GameplayAbilities/Interacts/Mount/BP_SlotBehavior_Mount.Car_OpenDoor_GetIn` _mountbehavior)))))

(fn `Get Mount Driver Thrown Out Montage`
  (returns (Car_GetInMontage :type "AnimMontage Object Reference"))
  (return (`/Game/Abilities/GameplayAbilities/Interacts/Mount/BP_SlotBehavior_Mount.Character_Carjack_PulledOut` (`self.MountBehavior`))))

(fn `GetMountSkeletalMesh`
  (params (`Pawn To Mount` :type "Actor Object Reference"))
  (returns (`Mesh Comp` :type "SkeletalMeshComponent Object Reference"))
  (bind _ascharacter (cast `Character` `Pawn To Mount`)
    (:`then`
      (return (`Character.Mesh` _ascharacter)))
    (:`CastFailed`
      (return (`|GetArrayItem` (`Actor.K2_GetComponentsByClass` `Pawn To Mount` "/Script/Engine.SkeletalMeshComponent") 1)))))

(fn `Grab Mount Data`
  (params (StoleFrom :type "NarrativeInteractionComponent Object Reference"))
  (returns (Succeeded :type Boolean) (FailReason :type String))
  (bind (_slotconfiguration_slottag _slotconfiguration_debugcolor _slotconfiguration_linkedslots _slotconfiguration_slottransform _slotconfiguration_slotinteractbehavior) (break `InteractionSlotConfig` (`self.SlotConfiguration`)))
  (bind _mountbehavior (`self.MountBehavior`))
  (bind (_interactionslotclaimhandle_handleindex _interactionslotclaimhandle_handleowner) (break `InteractionSlotClaimHandle` (`NarrativeInteractionComponent.InteractionSlotClaimHandle` (`self.InteractionComponent`))))
  (`/Engine/EditorBlueprintResources/StandardMacros.IsValid` StoleFrom
    (:`Is Valid`
      (bind _returnvalue (message `NarrativeCharacterOwner.GetNarrativeCharacter` (`NarrativeInteractionComponent.OwningController` StoleFrom)))
      (set `self.StealingFromPawn` _returnvalue))
    (:`Is Not Valid`
      (set `self.StealingFromPawn` null)))
  (set `self.OldController` (`Pawn.GetController` (`self.CharacterOwner`)))
  (set `self.OldCharacter` (`self.CharacterOwner`))
  (bind _asnarrative_npccharacter (cast `NarrativeNPCCharacter` (`self.CharacterOwner`))
    (:`then`
      (bind _asgoal_interact (cast `/Game/AI/Activities/Interact/Goals/Goal_Interact` (`NPCActivityComponent.GetCurrentActivityGoal` (`NarrativeNPCCharacter.GetActivityComponent` _asnarrative_npccharacter)))
        (:`then`
          (set `self.NPCInteractGoal` _asgoal_interact))
        (:`CastFailed`
          _)))
    (:`CastFailed`
      _))
  (bind _aspawn (cast `Pawn` (`ActorComponent.GetOwner` _interactionslotclaimhandle_handleowner))
    (:`then`
      (set `self.PawnToMount` _aspawn)
      (bind _asbp_slot_behavior_mount (cast `/Game/Abilities/GameplayAbilities/Interacts/Mount/BP_SlotBehavior_Mount` _slotconfiguration_slotinteractbehavior))
      (set `self.MountBehavior` _asbp_slot_behavior_mount)
      (if (and (`KismetSystemLibrary.IsValid` (`/Game/Abilities/GameplayAbilities/Interacts/Mount/BP_SlotBehavior_Mount.Character_GetOffMount` _mountbehavior)) (`KismetSystemLibrary.IsValid` (`/Game/Abilities/GameplayAbilities/Interacts/Mount/BP_SlotBehavior_Mount.Character_GetOnMount` _mountbehavior)))
        (return true "")
        (else
          (return false "GA_Interact_Mount failed -YourSit Down or Get Up Montage was null"))))
    (:`CastFailed`
      (return false "GA_Interact_Mount is supposed to be used with a pawn actor."))))

(fn `PossessMount`
  (locals (PreRot :type "Rotator Structure" :default (struct)))
  (if (`/Game/Abilities/GameplayAbilities/Interacts/Mount/BP_SlotBehavior_Mount.IsPassengerSlot` (`self.MountBehavior`))
    (`Controller.SetIgnoreMoveInput` (`self.OldController`) true)
    (else
      (set `local.PreRot` (`Controller.GetControlRotation` (`self.OldController`)))
      (`Controller.Possess` (`self.OldController`) (`self.PawnToMount`))
      (`Controller.SetControlRotation` (`self.OldController`) (`local.PreRot`)) ; Possession resets control rot which we dont want since we keep camera attached to main character
    ))
  (`NarrativeAnimInstance.ApplyOverrideLayer` (`NarrativeCharacter.GetCharacterAnimInstance` (`self.OldCharacter`)) (struct :`TagName` "Narrative.Anim.OverrideLayer.Driving") 0.0)
  (`PrimitiveComponent.SetCollisionEnabled` (`Character.CapsuleComponent` (`self.OldCharacter`)) "NoCollision") ; The pawn we possess may collide with us if we dont turn this off
  (`ActorComponent.SetTickGroup` (`Character.Mesh` (`self.OldCharacter`)) "TG_PostPhysics") ; We're now attached to something and our ABP needs to update after that does so things like car steering doesnt lag behind mesh
)

(fn `Ready Character For Warping`
  (params (`Character To Modify` :type "NarrativeCharacter Object Reference"))
  ; Modify the character such that we can motion warp it without collision etc glitching out
  (`Actor.K2_DetachFromActor` (`local.Character To Modify`) "KeepWorld" "KeepWorld" "KeepWorld") ; Detach if we're attached to anything
  (`PrimitiveComponent.SetCollisionEnabled` (`Character.CapsuleComponent` (`local.Character To Modify`)) "NoCollision") ; Query Only causes us to collide with CMC-based mounts like horses etc. This should be fine as mesh can still have collision so we should be able to take hits\nfrom people shooting us etc
  (`NarrativeCharacter.SetIgnoreActorWhenMoving` (`local.Character To Modify`) (`self.PawnToMount`) true)
  (`CharacterMovementComponent.SetMovementMode` (`Character.CharacterMovement` (`local.Character To Modify`)) "MOVE_Flying" 0))

(fn `Restore Character From Warping`
  (params (Character :type "NarrativeCharacter Object Reference"))
  ; Restore the character such that it is back to how it was prior to warp
  (`CharacterMovementComponent.SetMovementMode` (`Character.CharacterMovement` (`local.Character`)) "MOVE_Walking" 0)
  (`MotionWarpingComponent.RemoveWarpTarget` (`NarrativeCharacter.MotionWarpingComponent` (`local.Character`)) "SitWarp")
  (`PrimitiveComponent.IgnoreActorWhenMoving` (`Character.CapsuleComponent` (`local.Character`)) (`self.PawnToMount`) false)
  (`Actor.K2_DetachFromActor` (`local.Character`) "KeepWorld" "KeepWorld" "KeepWorld")
  (`PrimitiveComponent.SetCollisionEnabled` (`Character.CapsuleComponent` (`local.Character`)) "QueryAndPhysics"))

(fn `Started Entry Warp`)

(fn `Started Exit Warp`)

(fn `UnpossessMount`
  (locals (PreRot :type "Rotator Structure"))
  (bind _oldcharacter (`self.OldCharacter`))
  (bind _oldcontroller (`self.OldController`))
  (if (`/Game/Abilities/GameplayAbilities/Interacts/Mount/BP_SlotBehavior_Mount.IsPassengerSlot` (`self.MountBehavior`))
    (bind _asplayer_controller (cast `PlayerController` (`self.GetOwningController`))
      (:`then`
        (`Controller.SetIgnoreMoveInput` _asplayer_controller false)
        (`PlayerController.SetViewTargetWithBlend` _asplayer_controller (`self.OldCharacter`) 0.0 "VTBlend_Linear" 0.0 false))
      (:`CastFailed`
        _))
    (`ActorComponent.SetTickGroup` (`Character.Mesh` (`self.OldCharacter`)) "TG_PrePhysics" :!label _label) ; We're now attached to something and our ABP needs to update after that does so things like car steering doesnt lag behind mesh
    (else
      (set `local.PreRot` (`Controller.GetControlRotation` (`self.OldController`)))
      (if (!= (`Controller.K2_GetPawn` _oldcontroller) _oldcharacter)
        (`Controller.Possess` _oldcontroller _oldcharacter)
        (`Controller.SetControlRotation` (`self.OldController`) (`local.PreRot`)) ; Possession resets control rot which we dont want since we keep camera attached to main character
        (goto _label)))))