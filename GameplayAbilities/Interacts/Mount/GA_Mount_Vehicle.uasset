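; Gameplay ability for mounting and dismounting vehicles, specializing a parent mount interaction ability.
; It supplies the Narrative vehicle's skeletal mesh as the mount mesh.
; Overrides of the entry and exit warp hooks set the BP_VehicleBase handbrake when a warp starts and release it when it finishes.
; Interaction handling just defers to the parent, and a leftover node that enables mesh physics is never run.
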(event `self.HandleInteraction`
  (params (bIsStealing :type Boolean) (StealingFrom :type "NarrativeInteractionComponent Object Reference"))
  (`parent.HandleInteraction` bIsStealing StealingFrom))

(fn `Finished Entry Warp`
  (`parent.Finished Entry Warp`)
  (bind _pawntomount (`self.PawnToMount`)
    (:`then`
      (bind _asbp_vehicle_base (cast `/Game/Blueprints/Vehicles/Demo/Blueprint/BP_VehicleBase` _pawntomount))
      (`ChaosVehicleMovementComponent.SetHandbrakeInput` (`NarrativeWheeledVehicle.VehicleMovementComponent` _asbp_vehicle_base) false))
    (:`else`)))

(fn `Finished Exit Warp`
  (`parent.Finished Exit Warp`)
  (bind _pawntomount (`self.PawnToMount`)
    (:`then`
      (bind _asbp_vehicle_base (cast `/Game/Blueprints/Vehicles/Demo/Blueprint/BP_VehicleBase` _pawntomount))
      (`ChaosVehicleMovementComponent.SetHandbrakeInput` (`NarrativeWheeledVehicle.VehicleMovementComponent` _asbp_vehicle_base) false))
    (:`else`)))

(fn `GetMountSkeletalMesh`
  (params (`Pawn To Mount` :type "Actor Object Reference"))
  (returns (`Mesh Comp` :type "SkeletalMeshComponent Object Reference"))
  (bind _asnarrative_vehicle_base (cast `NarrativeVehicleBase` `Pawn To Mount`))
  (return (`NarrativeVehicleBase.Mesh` _asnarrative_vehicle_base)))

(fn `Started Entry Warp`
  (`parent.Started Entry Warp`)
  (bind _pawntomount (`self.PawnToMount`)
    (:`then`
      (bind _asbp_vehicle_base (cast `/Game/Blueprints/Vehicles/Demo/Blueprint/BP_VehicleBase` _pawntomount))
      (`ChaosVehicleMovementComponent.SetHandbrakeInput` (`NarrativeWheeledVehicle.VehicleMovementComponent` _asbp_vehicle_base) true))
    (:`else`)))

(fn `Started Exit Warp`
  (`parent.Started Exit Warp`)
  (bind _pawntomount (`self.PawnToMount`)
    (:`then`
      (bind _asbp_vehicle_base (cast `/Game/Blueprints/Vehicles/Demo/Blueprint/BP_VehicleBase` _pawntomount))
      (`ChaosVehicleMovementComponent.SetHandbrakeInput` (`NarrativeWheeledVehicle.VehicleMovementComponent` _asbp_vehicle_base) true))
    (:`else`)))