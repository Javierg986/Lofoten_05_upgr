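; Mount slot behavior for the interaction system, defining debug visualization and steal rules for mount slots.
; It draws a debug marker labeled as the get-out location, composing the get-out transform with the owner's transform.
; The stealable check calls the parent but always returns false, leaving the driver-only rule unhooked until pedestrian drivers exist, since quest partners and friendlies should not be jackable.
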(fn `GetDebugSlots`
  (params (SlotTransform :type "Transform Structure (by ref)") (OwnerTransform :type "Transform Structure (by ref)"))
  (returns (ReturnValue :type "Array of InteractionDebugVisualizeSlot Structure"))
  (locals (SlotColor :type "Color Structure" :default (struct :`B` 255 :`G` 162 :`A` 255)))
  (return (`|MakeArray` (make `InteractionDebugVisualizeSlot` (`KismetMathLibrary.ComposeTransforms` (`self.GetOutTransform`) OwnerTransform) (`local.SlotColor`) "Get Out Location"))))

(fn `IsStealable`
  (params (OurSlot :type Integer) (OurInteractable :type "NarrativeInteractableComponent Object Reference") (Interactor :type "NarrativeInteractionComponent Object Reference"))
  (returns (ReturnValue :type Boolean))
  (bind _returnvalue (`parent.IsStealable` OurSlot OurInteractable Interactor))
  (return false) ; Unhooked - when ped drivers are in we'll return true for that case - partners on quests etc and friendlies shouldnt be jackable
)