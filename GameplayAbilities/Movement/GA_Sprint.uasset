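; Gameplay ability that makes a Narrative character sprint while the input is held.
; Activation starts sprinting on the character's Narrative movement component and waits for input release, which ends the ability.
; A repeating task polls frequently and also ends it when the character leaves the ground or stops moving forward.
; Ending stops sprinting and cleans up the polling task.
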(event `self.K2_ActivateAbility`
  (bind _returnvalue (`NarrativeCharacter.GetNarrativeCharacterMovement` (`self.GetOwningNarrativeCharacter`)))
  ;[1 1 1] Crouch or uncrouch and end ability
  (`NarrativeCharacterMovement.StartSprinting` (`NarrativeCharacter.GetNarrativeCharacterMovement` (`self.GetOwningNarrativeCharacter`)))
  (`AbilityTask_WaitInputRelease.WaitInputRelease` true
    (:`then`
      (bind _asynctaskproxy (`AbilityTask_Repeat.RepeatAction` 0.1 99999)
        (:`then`
          (set `self.RepeatTask` _asynctaskproxy))
        (:`OnPerformAction`
          (if (or (not (`NavMovementComponent.IsMovingOnGround` _returnvalue)) (not (`NarrativeCharacterMovement.IsMovingForward` _returnvalue 2.0)))
            (`self.K2_EndAbility`)))))
    (:`OnRelease`
      (`self.K2_EndAbility`))))

(event `self.K2_OnEndAbility`
  (params (bWasCancelled :type Boolean))
  ;[1 1 1] Crouch or uncrouch and end ability
  (`NarrativeCharacterMovement.StopSprinting` (`NarrativeCharacter.GetNarrativeCharacterMovement` (`self.GetOwningNarrativeCharacter`)))
  (bind _repeattask (`self.RepeatTask`)
    (:`then`
      (`GameplayTask.EndTask` _repeattask))
    (:`else`)))